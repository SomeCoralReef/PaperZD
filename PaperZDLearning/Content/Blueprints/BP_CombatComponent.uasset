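; BP_CombatComponent is a unit's combat component, scheduling when its owning BP_UnitBase asks for a battle turn.
; On BeginPlay it stores the unit and its transform as the battle position, then starts a one-shot action timer that shortens as Haste rises.
; When the timer fires, RequestTurn passes the unit to BP_BattleGameMode's TurnRequest.
; StartUnitTurn and EndUnitTurn are empty stubs.
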(event EventBeginPlay
  (bind _asbp_unit_base (Utilities|Casting|CastToBP_UnitBase (Components|GetOwner)))
  (bind _output_get (Variables|Default|SetUnitCharacter _asbp_unit_base))
  (Variables|Default|SetBattlePosition (Transformation|GetActorTransform _output_get))
  (CallFunction|BeginBattle))

(event EventTick
  (params (DeltaSeconds :type Float%20%28single-precision%29)))

(fn StartUnitTurn)

(fn EndUnitTurn)

(fn BeginBattle
  (bind _returnvalue (Utilities|Time|SetTimerbyFunctionName self "RequestTurn" (+ (* (- 1.0 (Math|Float|NormalizetoRange (Variables|UnitStats|GetHaste) 0.0 255.0)) (Variables|Default|GetMaxActionTime)) (Variables|Default|GetMinActionTime))))
  (Variables|Default|SetActionTimer _returnvalue))

(fn RequestTurn
  (bind _asbp_battle_game_mode (Utilities|Casting|CastToBP_BattleGameMode (Game|GetGameMode)))
  (Default|TurnRequest _asbp_battle_game_mode (Variables|Default|GetUnitCharacter)))